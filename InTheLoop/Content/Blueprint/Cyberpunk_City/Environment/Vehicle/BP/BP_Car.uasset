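; BP_Car is a vehicle actor that drives itself along a spline path in the Cyberpunk City environment.
; On BeginPlay it finds a BP_CarSplinePath_01 actor in the level by class and calls Move.
; Move plays the MoveCar timeline at a rate of one over TimeToComplete.
; Each update maps the CarTrack value to distance along the spline and sets the car's world location and rotation from it.
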(event Custom|Move
  (bind _splineref (Variables|Default|GetSplineREF))
  (bind _spline (Variables|/Game/Blueprint/Cyberpunk_City/Environment/Vehicle/BP/BP_CarSplinePath_01.BP_CarSplinePath_01_C|GetSpline _splineref))
  (Components|Timeline|SetPlayRate (Variables|Default|GetMove%20Car) (/ 1.0 (Variables|Default|GetTime%20to%20Complete)))
  (bind _cartrack (Timeline|Move%20Car Play)
    (:Update
      (Transformation|SetActorTransform (Math|Transform|MakeTransform (Spline|GetLocationatDistanceAlongSpline _spline (Math|Float|Lerp 0.0 (Spline|GetSplineLength (Variables|/Game/Blueprint/Cyberpunk_City/Environment/Vehicle/BP/BP_CarSplinePath_01.BP_CarSplinePath_01_C|GetSpline (Variables|Default|GetSplineREF))) _cartrack) "World") (Spline|GetRotationatDistanceAlongSpline _spline (Math|Float|Lerp 0.0 (Spline|GetSplineLength (Variables|/Game/Blueprint/Cyberpunk_City/Environment/Vehicle/BP/BP_CarSplinePath_01.BP_CarSplinePath_01_C|GetSpline (Variables|Default|GetSplineREF))) _cartrack) "World") "1.000000,1.000000,1.000000")))))

(event EventBeginPlay
  (bind _returnvalue (Actor|GetActorOfClass "/Game/Blueprint/Cyberpunk_City/Environment/Vehicle/BP/BP_CarSplinePath_01.BP_CarSplinePath_01_C"))
  (Variables|Default|SetSplineREF _returnvalue)
  (CallFunction|Move))

(fn ConstructionScript)