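; Trigger volume that delivers the next scripted chat message to the player's chat widget when the first-person character overlaps its Box.
; ObjectIndex selects one of four chat slots, plays a sound, shows its new-message indicator and, if text differs, sets message and replies from indexed arrays, then advances the index.
; Slot 3 reuses slot 2's reply fields and arrays; slot 4 sets no replies.
; The widget created on BeginPlay is never used.
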(event OnComponentBeginOverlap(Box)
  (params (OverlappedComponent :type Primitive%20Component%20Object%20Reference) (OtherActor :type Actor%20Object%20Reference) (OtherComp :type Primitive%20Component%20Object%20Reference) (OtherBodyIndex :type Integer) (bFromSweep :type Boolean) (SweepResult :type Hit%20Result%20Structure%20%28by%20ref%29))
  (bind _returnvalue (Game|GetPlayerCharacter 0))
  (bind _asbp_first_person_character (Utilities|Casting|CastToBP_FirstPersonCharacter _returnvalue))
  (bind _chat (Variables|/Game/FirstPerson/Blueprints/BP_FirstPersonCharacter.BP_FirstPersonCharacter_C|GetChat _asbp_first_person_character))
  (bind _chat_2 (Variables|/Game/FirstPerson/Blueprints/BP_FirstPersonCharacter.BP_FirstPersonCharacter_C|GetChat _asbp_first_person_character))
  (bind _chat_3 (Variables|/Game/FirstPerson/Blueprints/BP_FirstPersonCharacter.BP_FirstPersonCharacter_C|GetChat _asbp_first_person_character))
  (bind _chat_4 (Variables|/Game/FirstPerson/Blueprints/BP_FirstPersonCharacter.BP_FirstPersonCharacter_C|GetChat _asbp_first_person_character))
  (bind _t_object1 (Variables|/Game/Blueprint/UI/WB_Drag_Chat_5.WB_Drag_Chat_5_C|GetT_Object1 _chat_2))
  (bind _t_object2 (Variables|/Game/Blueprint/UI/WB_Drag_Chat_5.WB_Drag_Chat_5_C|GetT_Object2 _chat_3))
  (bind _t_object3 (Variables|/Game/Blueprint/UI/WB_Drag_Chat_5.WB_Drag_Chat_5_C|GetT_Object3 _chat_4))
  (bind _t_object4 (Variables|/Game/Blueprint/UI/WB_Drag_Chat_5.WB_Drag_Chat_5_C|GetT_Object4 _chat))
  (bind _text (Variables|/Script/UMG.TextBlock|GetText _t_object1))
  (bind _text_2 (Variables|/Script/UMG.TextBlock|GetText _t_object2))
  (bind _text_3 (Variables|/Script/UMG.TextBlock|GetText _t_object4))
  (bind _text_4 (Variables|/Script/UMG.TextBlock|GetText _t_object3))
  ;[0.15 0.15 0.15 0.5] Comment
  (Utilities|IsValid _asbp_first_person_character
    (:Is%20Valid
      (if (== OtherActor _asbp_first_person_character)
        (switch int (Variables|Default|GetObjectIndex)
          (:1
            ;;[0.15 0.15 0.15 0.5] Object1 Message Text
            (Audio|PlaySound2D 0 1.0 1.0 0.0 0 0)
            (Widget|SetVisibility (Variables|/Game/Blueprint/UI/WB_Drag_Chat_5.WB_Drag_Chat_5_C|GetObject_NewMessage1 _chat_2) "Visible")
            (Variables|Object1|SetCurrentText1 _text)
            (if (not (Utilities|Enum|Equal(Enum) _text (Utilities|Array|Get(acopy) (Variables|Object1|GetNewText1) (Variables|Object1|GetTextIndex1))))
              (Rendering|Components|TextRender|SetText _t_object1 (Utilities|Array|Get(acopy) (Variables|Object1|GetNewText1) (Variables|Object1|GetTextIndex1)))
              (Rendering|Components|TextRender|SetText (Variables|/Game/Blueprint/UI/WB_Drag_Chat_5.WB_Drag_Chat_5_C|GetT1_Object _chat_2) (Utilities|Array|Get(acopy) (Variables|Object1|GetNewText1) (Variables|Object1|GetTextIndex1)))
              ;;[0.15 0.15 0.15 0.5] Response
              (Rendering|Components|TextRender|SetText (Variables|/Game/Blueprint/UI/WB_Drag_Chat_5.WB_Drag_Chat_5_C|GetT_Option1A _chat_2) (Utilities|Array|Get(acopy) (Variables|Object1|GetNewOptionText1A) (Variables|Object1|GetTextIndex1)))
              (Rendering|Components|TextRender|SetText (Variables|/Game/Blueprint/UI/WB_Drag_Chat_5.WB_Drag_Chat_5_C|GetT_Option1B _chat_2) (Utilities|Array|Get(acopy) (Variables|Object1|GetNewOptionText1B) (Variables|Object1|GetTextIndex1)))
              (Rendering|Components|TextRender|SetText (Variables|/Game/Blueprint/UI/WB_Drag_Chat_5.WB_Drag_Chat_5_C|GetT_Option1C _chat_2) (Utilities|Array|Get(acopy) (Variables|Object1|GetNewOptionText1C) (Variables|Object1|GetTextIndex1)))
              (Rendering|Components|TextRender|SetText (Variables|/Game/Blueprint/UI/WB_Drag_Chat_5.WB_Drag_Chat_5_C|GetT_Option1D _chat_2) (Utilities|Array|Get(acopy) (Variables|Object1|GetNewOptionText1D) (Variables|Object1|GetTextIndex1)))
              (bind _result (Math|Integer|IncrementInt (Variables|Object1|GetTextIndex1))
                (:%20%20
                  (Variables|Object1|SetTextIndex1 _result)))))
          (:2
            (Audio|PlaySound2D 0 1.0 1.0 0.0 0 0)
            (Widget|SetVisibility (Variables|/Game/Blueprint/UI/WB_Drag_Chat_5.WB_Drag_Chat_5_C|GetObject_NewMessage2 _chat_3) "Visible")
            (Variables|Object2|SetCurrentText2 _text_2)
            (if (not (Utilities|Enum|Equal(Enum) _text_2 (Utilities|Array|Get(acopy) (Variables|Object2|GetNewText2) (Variables|Object2|GetTextIndex2))))
              (Rendering|Components|TextRender|SetText _t_object2 (Utilities|Array|Get(acopy) (Variables|Object2|GetNewText2) (Variables|Object2|GetTextIndex2)))
              (Rendering|Components|TextRender|SetText (Variables|/Game/Blueprint/UI/WB_Drag_Chat_5.WB_Drag_Chat_5_C|GetT2_Object _chat_3) (Utilities|Array|Get(acopy) (Variables|Object2|GetNewText2) (Variables|Object2|GetTextIndex2)))
              ;;[0.15 0.15 0.15 0.5] Response
              (Rendering|Components|TextRender|SetText (Variables|/Game/Blueprint/UI/WB_Drag_Chat_5.WB_Drag_Chat_5_C|GetT_Option2A _chat_3) (Utilities|Array|Get(acopy) (Variables|Object2|GetNewOptionText2A) (Variables|Object2|GetTextIndex2)))
              (Rendering|Components|TextRender|SetText (Variables|/Game/Blueprint/UI/WB_Drag_Chat_5.WB_Drag_Chat_5_C|GetT_Option2B _chat_3) (Utilities|Array|Get(acopy) (Variables|Object2|GetNewOptionText2B) (Variables|Object2|GetTextIndex2)))
              (Rendering|Components|TextRender|SetText (Variables|/Game/Blueprint/UI/WB_Drag_Chat_5.WB_Drag_Chat_5_C|GetT_Option2C _chat_3) (Utilities|Array|Get(acopy) (Variables|Object2|GetNewOptionText2C) (Variables|Object2|GetTextIndex2)))
              (Rendering|Components|TextRender|SetText (Variables|/Game/Blueprint/UI/WB_Drag_Chat_5.WB_Drag_Chat_5_C|GetT_Option2D _chat_3) (Utilities|Array|Get(acopy) (Variables|Object2|GetNewOptionText2D) (Variables|Object2|GetTextIndex2)))
              (bind _result_2 (Math|Integer|IncrementInt (Variables|Object2|GetTextIndex2))
                (:%20%20
                  (Variables|Object2|SetTextIndex2 _result_2)))))
          (:3
            (Audio|PlaySound2D 0 1.0 1.0 0.0 0 0)
            (Widget|SetVisibility (Variables|/Game/Blueprint/UI/WB_Drag_Chat_5.WB_Drag_Chat_5_C|GetObject_NewMessage3 _chat_4) "Visible")
            (Variables|Object3|SetCurrentText3 _text_4)
            (if (not (Utilities|Enum|Equal(Enum) _text_4 (Utilities|Array|Get(acopy) (Variables|Object3|GetNewText3) (Variables|Object3|GetTextIndex3))))
              (Rendering|Components|TextRender|SetText _t_object3 (Utilities|Array|Get(acopy) (Variables|Object3|GetNewText3) (Variables|Object3|GetTextIndex3)))
              (Rendering|Components|TextRender|SetText (Variables|/Game/Blueprint/UI/WB_Drag_Chat_5.WB_Drag_Chat_5_C|GetT3_Object _chat_4) (Utilities|Array|Get(acopy) (Variables|Object3|GetNewText3) (Variables|Object3|GetTextIndex3)))
              ;;[0.15 0.15 0.15 0.5] Response
              (Rendering|Components|TextRender|SetText (Variables|/Game/Blueprint/UI/WB_Drag_Chat_5.WB_Drag_Chat_5_C|GetT_Option2A _chat_4) (Utilities|Array|Get(acopy) (Variables|Object2|GetNewOptionText2A) (Variables|Object3|GetTextIndex3)))
              (Rendering|Components|TextRender|SetText (Variables|/Game/Blueprint/UI/WB_Drag_Chat_5.WB_Drag_Chat_5_C|GetT_Option2B _chat_4) (Utilities|Array|Get(acopy) (Variables|Object2|GetNewOptionText2B) (Variables|Object3|GetTextIndex3)))
              (Rendering|Components|TextRender|SetText (Variables|/Game/Blueprint/UI/WB_Drag_Chat_5.WB_Drag_Chat_5_C|GetT_Option2C _chat_4) (Utilities|Array|Get(acopy) (Variables|Object2|GetNewOptionText2C) (Variables|Object3|GetTextIndex3)))
              (Rendering|Components|TextRender|SetText (Variables|/Game/Blueprint/UI/WB_Drag_Chat_5.WB_Drag_Chat_5_C|GetT_Option2D _chat_4) (Utilities|Array|Get(acopy) (Variables|Object2|GetNewOptionText2D) (Variables|Object3|GetTextIndex3)))
              (bind _result_3 (Math|Integer|IncrementInt (Variables|Object3|GetTextIndex3))
                (:%20%20
                  (Variables|Object3|SetTextIndex3 _result_3)))))
          (:4
            (Audio|PlaySound2D 0 1.0 1.0 0.0 0 0)
            (Widget|SetVisibility (Variables|/Game/Blueprint/UI/WB_Drag_Chat_5.WB_Drag_Chat_5_C|GetObject_NewMessage4 _chat) "Visible")
            (Variables|Object4|SetCurrentText4 _text_3)
            (if (not (Utilities|Enum|Equal(Enum) _text_3 (Utilities|Array|Get(acopy) (Variables|Object4|GetNewText4) (Variables|Object4|GetTextIndex4))))
              (Rendering|Components|TextRender|SetText _t_object4 (Utilities|Array|Get(acopy) (Variables|Object4|GetNewText4) (Variables|Object4|GetTextIndex4)))
              (Rendering|Components|TextRender|SetText (Variables|/Game/Blueprint/UI/WB_Drag_Chat_5.WB_Drag_Chat_5_C|GetT4_Object _chat) (Utilities|Array|Get(acopy) (Variables|Object4|GetNewText4) (Variables|Object4|GetTextIndex4)))
              (bind _result_4 (Math|Integer|IncrementInt (Variables|Object4|GetTextIndex4))
                (:%20%20
                  (Variables|Object4|SetTextIndex4 _result_4))))))))))

(event EventBeginPlay
  (bind _returnvalue (UserInterface|CreateWidget "/Game/Blueprint/UI/WB_Drag_Chat_5.WB_Drag_Chat_5_C"))
  (Variables|Default|SetChat _returnvalue))

(event Collision|EventActorBeginOverlap
  (params (OtherActor :type Actor%20Object%20Reference)))

(event EventTick
  (params (DeltaSeconds :type Float%20%28single-precision%29))
  ;[0.15 0.15 0.15 0.5] Comment
)

(fn ConstructionScript)