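; Trigger actor that pops up a random UI window on screen when the first-person player character enters its Box.
; Each overlap picks a widget class from the UI array using a random index up to RangeMax, then creates it for the first player.
; The widget gets a random position within fixed pixel bounds before being added to the viewport.
; Nothing live removes the widgets; the removal and RandomPosition nodes are unconnected leftovers.
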(event OnComponentBeginOverlap(Box)
  (params (OverlappedComponent :type Primitive%20Component%20Object%20Reference) (OtherActor :type Actor%20Object%20Reference) (OtherComp :type Primitive%20Component%20Object%20Reference) (OtherBodyIndex :type Integer) (bFromSweep :type Boolean) (SweepResult :type Hit%20Result%20Structure%20%28by%20ref%29))
  ;[0.15 0.15 0.15 0.5] Comment
  (if (== OtherActor (.AsBP%20First%20Person%20Character (Utilities|Casting|CastToBP_FirstPersonCharacter (Game|GetPlayerCharacter 0))))
    (bind _returnvalue (UserInterface|CreateWidget (Utilities|Array|Get(acopy) (Variables|Default|GetUI) (Math|Random|RandomIntegerinRange 0 (Variables|Default|GetRangeMax))) (Game|GetPlayerController 0)))
    (Class|UserWidget|SetPositioninViewport _returnvalue (Math|Vector2D|MakeVector2D (Math|Random|RandomFloatinRange 2e+02 3.5e+03) (Math|Random|RandomFloatinRange 1e+02 9.8e+02)) true)
    (UserInterface|Viewport|AddtoViewport _returnvalue 0)))

(event EventBeginPlay)

(event Collision|EventActorBeginOverlap
  (params (OtherActor :type Actor%20Object%20Reference)))

(event EventTick
  (params (DeltaSeconds :type Float%20%28single-precision%29)))

(fn ConstructionScript)