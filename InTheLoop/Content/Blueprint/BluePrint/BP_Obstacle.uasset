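; BP_Obstacle is an obstacle actor that costs the first-person player time on contact.
; When the player character begins overlapping its Box, it subtracts a fixed amount from the character's Time variable.
; A DoOnce gate blocks repeat penalties until a short delay after the player leaves the box.
; BeginPlay also creates and stores a WB_MainView widget, which the graph never displays or uses.
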(event OnComponentBeginOverlap(Box)
  (params (OverlappedComponent :type Primitive%20Component%20Object%20Reference) (OtherActor :type Actor%20Object%20Reference) (OtherComp :type Primitive%20Component%20Object%20Reference) (OtherBodyIndex :type Integer) (bFromSweep :type Boolean) (SweepResult :type Hit%20Result%20Structure%20%28by%20ref%29))
  (bind _returnvalue (Game|GetPlayerCharacter 0))
  (bind _returnvalue_2 (Game|GetPlayerCharacter 0))
  (bind _asbp_first_person_character (Utilities|Casting|CastToBP_FirstPersonCharacter _returnvalue_2))
  (bind _asbp_first_person_character_2 (Utilities|Casting|CastToBP_FirstPersonCharacter _returnvalue))
  ;[0.15 0.15 0.15 0.5] Comment
  (Utilities|IsValid _asbp_first_person_character_2
    (:Is%20Valid
      (if (== OtherActor _asbp_first_person_character_2)
        (Utilities|FlowControl|DoOnce false
          (:Completed
            (Variables|/Game/FirstPerson/Blueprints/BP_FirstPersonCharacter.BP_FirstPersonCharacter_C|Settime _asbp_first_person_character (- (Variables|/Game/FirstPerson/Blueprints/BP_FirstPersonCharacter.BP_FirstPersonCharacter_C|Gettime _asbp_first_person_character) 1e+01))))))))

(event OnComponentEndOverlap(Box)
  (params (OverlappedComponent :type Primitive%20Component%20Object%20Reference) (OtherActor :type Actor%20Object%20Reference) (OtherComp :type Primitive%20Component%20Object%20Reference) (OtherBodyIndex :type Integer))
  (bind _returnvalue (Game|GetPlayerCharacter 0))
  (bind _returnvalue_2 (Game|GetPlayerCharacter 0))
  (bind _asbp_first_person_character (Utilities|Casting|CastToBP_FirstPersonCharacter _returnvalue))
  (bind _asbp_first_person_character_2 (Utilities|Casting|CastToBP_FirstPersonCharacter _returnvalue_2))
  ;[0.15 0.15 0.15 0.5] Comment
  (Utilities|IsValid _asbp_first_person_character
    (:Is%20Valid
      (if (== OtherActor _asbp_first_person_character)
        (Utilities|FlowControl|Delay 1.0)
        (Utilities|FlowControl|DoOnce false) ; enters at Reset
      ))))

(event EventBeginPlay
  ;[0.15 0.15 0.15 0.5] Comment
  (bind _returnvalue (UserInterface|CreateWidget "/Game/Blueprint/UI/WB_MainView.WB_MainView_C"))
  (Variables|Default|SetMain _returnvalue))

(event Collision|EventActorBeginOverlap
  (params (OtherActor :type Actor%20Object%20Reference)))

(fn ConstructionScript)