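; Car Blueprint that drives along a referenced track's spline and costs the first-person player time on contact.
; A timeline alpha maps to spline distance to set location and rotation, with play rate from Duration and a start offset.
; RedLight plays the timeline and GreenLight stops it.
; Box overlap subtracts from the player's Time through a DoOnce, which resets shortly after the player leaves.
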(event OnComponentBeginOverlap(Box)
  (params (OverlappedComponent :type Primitive%20Component%20Object%20Reference) (OtherActor :type Actor%20Object%20Reference) (OtherComp :type Primitive%20Component%20Object%20Reference) (OtherBodyIndex :type Integer) (bFromSweep :type Boolean) (SweepResult :type Hit%20Result%20Structure%20%28by%20ref%29))
  (bind _returnvalue (Game|GetPlayerCharacter 0))
  (bind _returnvalue_2 (Game|GetPlayerCharacter 0))
  (bind _asbp_first_person_character (Utilities|Casting|CastToBP_FirstPersonCharacter _returnvalue_2))
  (bind _asbp_first_person_character_2 (Utilities|Casting|CastToBP_FirstPersonCharacter _returnvalue))
  (Utilities|IsValid _asbp_first_person_character_2
    (:Is%20Valid
      (if (== OtherActor _asbp_first_person_character_2)
        (Utilities|FlowControl|DoOnce false
          (:Completed
            (Variables|/Game/FirstPerson/Blueprints/BP_FirstPersonCharacter.BP_FirstPersonCharacter_C|Settime _asbp_first_person_character (- (Variables|/Game/FirstPerson/Blueprints/BP_FirstPersonCharacter.BP_FirstPersonCharacter_C|Gettime _asbp_first_person_character) 1e+01))))))))

(event OnComponentEndOverlap(Box)
  (params (OverlappedComponent :type Primitive%20Component%20Object%20Reference) (OtherActor :type Actor%20Object%20Reference) (OtherComp :type Primitive%20Component%20Object%20Reference) (OtherBodyIndex :type Integer))
  (bind _returnvalue (Game|GetPlayerCharacter 0))
  (bind _returnvalue_2 (Game|GetPlayerCharacter 0))
  (bind _asbp_first_person_character (Utilities|Casting|CastToBP_FirstPersonCharacter _returnvalue))
  (bind _asbp_first_person_character_2 (Utilities|Casting|CastToBP_FirstPersonCharacter _returnvalue_2))
  (Utilities|IsValid _asbp_first_person_character
    (:Is%20Valid
      (if (== OtherActor _asbp_first_person_character)
        (Utilities|FlowControl|Delay 1.0)
        (Utilities|FlowControl|DoOnce false) ; enters at Reset
      ))))

(event Custom|Move_Car
  (Components|Timeline|SetPlayRate (Variables|Default|GetCar_Mover) (/ 1.0 (Variables|Default|GetDuration)))
  (Components|Timeline|SetNewTime (Variables|Default|GetCar_Mover) (Variables|Default|GetCar_Start_Offset))
  (bind _alpha (Timeline|Car_Mover Play)
    (:Update
      (Variables|Default|SetAlpha _alpha)
      (Transformation|SetActorLocationAndRotation (Spline|GetLocationatDistanceAlongSpline (Variables|/Game/Blueprint/Station_Bravo/Blueprints/BP_Car_Track.BP_Car_Track_C|GetCar_Spline (Variables|Default|GetTrack_Reference)) (Math|Float|Lerp 0.0 (Spline|GetSplineLength (Variables|/Game/Blueprint/Station_Bravo/Blueprints/BP_Car_Track.BP_Car_Track_C|GetCar_Spline (Variables|Default|GetTrack_Reference))) (Variables|Default|GetAlpha)) "World") (Spline|GetRotationatDistanceAlongSpline (Variables|/Game/Blueprint/Station_Bravo/Blueprints/BP_Car_Track.BP_Car_Track_C|GetCar_Spline (Variables|Default|GetTrack_Reference)) (Math|Float|Lerp 0.0 (Spline|GetSplineLength (Variables|/Game/Blueprint/Station_Bravo/Blueprints/BP_Car_Track.BP_Car_Track_C|GetCar_Spline (Variables|Default|GetTrack_Reference))) (Variables|Default|GetAlpha)) "World")))))

(event Custom|RedLight
  (bind _alpha (Timeline|Car_Mover Play)
    (:Update
      (Variables|Default|SetAlpha _alpha)
      (Transformation|SetActorLocationAndRotation (Spline|GetLocationatDistanceAlongSpline (Variables|/Game/Blueprint/Station_Bravo/Blueprints/BP_Car_Track.BP_Car_Track_C|GetCar_Spline (Variables|Default|GetTrack_Reference)) (Math|Float|Lerp 0.0 (Spline|GetSplineLength (Variables|/Game/Blueprint/Station_Bravo/Blueprints/BP_Car_Track.BP_Car_Track_C|GetCar_Spline (Variables|Default|GetTrack_Reference))) (Variables|Default|GetAlpha)) "World") (Spline|GetRotationatDistanceAlongSpline (Variables|/Game/Blueprint/Station_Bravo/Blueprints/BP_Car_Track.BP_Car_Track_C|GetCar_Spline (Variables|Default|GetTrack_Reference)) (Math|Float|Lerp 0.0 (Spline|GetSplineLength (Variables|/Game/Blueprint/Station_Bravo/Blueprints/BP_Car_Track.BP_Car_Track_C|GetCar_Spline (Variables|Default|GetTrack_Reference))) (Variables|Default|GetAlpha)) "World")))))

(event Custom|GreenLight
  (bind _alpha (Timeline|Car_Mover Stop)
    (:Update
      (Variables|Default|SetAlpha _alpha)
      (Transformation|SetActorLocationAndRotation (Spline|GetLocationatDistanceAlongSpline (Variables|/Game/Blueprint/Station_Bravo/Blueprints/BP_Car_Track.BP_Car_Track_C|GetCar_Spline (Variables|Default|GetTrack_Reference)) (Math|Float|Lerp 0.0 (Spline|GetSplineLength (Variables|/Game/Blueprint/Station_Bravo/Blueprints/BP_Car_Track.BP_Car_Track_C|GetCar_Spline (Variables|Default|GetTrack_Reference))) (Variables|Default|GetAlpha)) "World") (Spline|GetRotationatDistanceAlongSpline (Variables|/Game/Blueprint/Station_Bravo/Blueprints/BP_Car_Track.BP_Car_Track_C|GetCar_Spline (Variables|Default|GetTrack_Reference)) (Math|Float|Lerp 0.0 (Spline|GetSplineLength (Variables|/Game/Blueprint/Station_Bravo/Blueprints/BP_Car_Track.BP_Car_Track_C|GetCar_Spline (Variables|Default|GetTrack_Reference))) (Variables|Default|GetAlpha)) "World")))))

(event Custom|StartCar
  (if (Variables|Default|GetCar_On/Off)
    (CallFunction|MoveCar)))

(event EventBeginPlay)

(fn ConstructionScript)