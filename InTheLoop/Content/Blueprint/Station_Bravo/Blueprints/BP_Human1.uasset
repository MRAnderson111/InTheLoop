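; Passerby NPC for Station Bravo that walks between patrol points and costs the player time on contact.
; On BeginPlay it gathers patrol point actors, and RandomMove chains AI MoveTo calls through them in array order, without randomizing or looping.
; Player capsule overlap halts it, then a DoOnce-gated branch plays a sound, deducts character Time and resumes walking after a delay.
; The gate resets shortly after overlap ends.
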(event OnComponentBeginOverlap(Capsule)
  (params (OverlappedComponent :type Primitive%20Component%20Object%20Reference) (OtherActor :type Actor%20Object%20Reference) (OtherComp :type Primitive%20Component%20Object%20Reference) (OtherBodyIndex :type Integer) (bFromSweep :type Boolean) (SweepResult :type Hit%20Result%20Structure%20%28by%20ref%29))
  (bind _returnvalue (Game|GetPlayerCharacter 0))
  (bind _asbp_first_person_character (Utilities|Casting|CastToBP_FirstPersonCharacter _returnvalue))
  ;[0.15 0.15 0.15 0.5] Comment
  (if (== OtherActor (.AsBP%20First%20Person%20Character (Utilities|Casting|CastToBP_FirstPersonCharacter (Game|GetPlayerCharacter 0))))
    (Components|Movement|StopMovementImmediately (Variables|Character|GetCharacterMovement self))
    (Utilities|FlowControl|DoOnce false
      (:Completed
        (Audio|PlaySound2D "/Game/SFX/Passerby_SoundCue.Passerby_SoundCue" 1.0 1.0 0.0 0 0)
        (Variables|/Game/FirstPerson/Blueprints/BP_FirstPersonCharacter.BP_FirstPersonCharacter_C|Settime _asbp_first_person_character (Utilities|Operators|Subtract (Variables|/Game/FirstPerson/Blueprints/BP_FirstPersonCharacter.BP_FirstPersonCharacter_C|Gettime _asbp_first_person_character) 1e+01))
        (Utilities|FlowControl|Delay 2.0)
        (CallFunction|RandomMove)))))

(event OnComponentEndOverlap(Capsule)
  (params (OverlappedComponent :type Primitive%20Component%20Object%20Reference) (OtherActor :type Actor%20Object%20Reference) (OtherComp :type Primitive%20Component%20Object%20Reference) (OtherBodyIndex :type Integer))
  (bind _returnvalue (Game|GetPlayerCharacter 0))
  (bind _asbp_first_person_character (Utilities|Casting|CastToBP_FirstPersonCharacter _returnvalue))
  ;[0.15 0.15 0.15 0.5] Comment
  (if (== OtherActor (.AsBP%20First%20Person%20Character (Utilities|Casting|CastToBP_FirstPersonCharacter (Game|GetPlayerCharacter 0))))
    (Utilities|FlowControl|Delay 1.0)
    (Utilities|FlowControl|DoOnce false) ; enters at Reset
  ))

(event Custom|RandomMove
  ;[0.15 0.15 0.15 0.5] Comment
  (AI|AIMoveTo self (Transformation|GetActorLocation (Utilities|Array|Get(acopy) (stale EventBeginPlay _output_get) (Variables|Default|GetPPIndex))) 0 5.0 false
    (:OnSuccess
      (Utilities|FlowControl|Delay 0.1)
      (if (not (>= (Variables|Default|GetPPIndex) (Utilities|Array|Length (stale EventBeginPlay _output_get))))
        (bind _result (Math|Integer|IncrementInt (Variables|Default|GetPPIndex))
          (:%20%20
            (Variables|Default|SetPPIndex _result)
            (CallFunction|RandomMove)))))))

(event EventBeginPlay
  ;[0.15 0.15 0.15 0.5] Comment
  (bind _returnvalue (UserInterface|CreateWidget "/Game/Blueprint/UI/WB_MainView.WB_MainView_C"))
  (Variables|Default|SetMain _returnvalue)
  (bind _asbp_patrol_point (Utilities|Casting|CastToBP_PatrolPointClass "/Game/Blueprint/PatrolPoint/BP_PatrolPoint.BP_PatrolPoint_C"))
  (bind _outactors (Actor|GetAllActorsOfClass _asbp_patrol_point))
  (bind _output_get (Variables|Default|SetPatrolPoint _outactors))
  (CallFunction|RandomMove))

(event Collision|EventActorBeginOverlap
  (params (OtherActor :type Actor%20Object%20Reference)))

(event EventTick
  (params (DeltaSeconds :type Float%20%28single-precision%29)))

(fn ConstructionScript)