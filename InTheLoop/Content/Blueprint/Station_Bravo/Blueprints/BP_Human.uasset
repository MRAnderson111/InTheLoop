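; BP_Human is a patrolling NPC that reacts when the player touches it.
; On BeginPlay it creates a WB_MainView widget and gathers all BP_PatrolPoint actors.
; Despite its name, RandomMove visits points in array order via AIMoveTo, pausing between them, with no index wrap or failure handling.
; Player capsule overlap stops movement, calls the widget's Minues, prints a message and resumes after a delay; end overlap calls Restore.
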(event OnComponentEndOverlap(Capsule)
  (params (OverlappedComponent :type Primitive%20Component%20Object%20Reference) (OtherActor :type Actor%20Object%20Reference) (OtherComp :type Primitive%20Component%20Object%20Reference) (OtherBodyIndex :type Integer))
  ;[0.15 0.15 0.15 0.5] Comment
  (if (== OtherActor (.AsBP%20First%20Person%20Character (Utilities|Casting|CastToBP_FirstPersonCharacter (Game|GetPlayerCharacter 0))))
    (Default|Restore (Variables|Default|GetMain))))

(event OnComponentBeginOverlap(Capsule)
  (params (OverlappedComponent :type Primitive%20Component%20Object%20Reference) (OtherActor :type Actor%20Object%20Reference) (OtherComp :type Primitive%20Component%20Object%20Reference) (OtherBodyIndex :type Integer) (bFromSweep :type Boolean) (SweepResult :type Hit%20Result%20Structure%20%28by%20ref%29))
  ;[0.15 0.15 0.15 0.5] Comment
  (if (== OtherActor (.AsBP%20First%20Person%20Character (Utilities|Casting|CastToBP_FirstPersonCharacter (Game|GetPlayerCharacter 0))))
    (Components|Movement|StopMovementImmediately (Variables|Character|GetCharacterMovement self))
    (Default|Minues (Variables|Default|GetMain))
    (Development|PrintString "Fuck Out")
    (Utilities|FlowControl|Delay 2.0)
    (CallFunction|RandomMove)))

(event Custom|RandomMove
  ;[0.15 0.15 0.15 0.5] Comment
  (AI|AIMoveTo self (Transformation|GetActorLocation (Utilities|Array|Get(acopy) (stale EventBeginPlay _output_get) (Variables|Default|GetPPIndex))) 0 5.0 false
    (:OnSuccess
      (Utilities|FlowControl|Delay 3.0)
      (bind _result (Math|Integer|IncrementInt (Variables|Default|GetPPIndex))
        (:%20%20
          (Variables|Default|SetPPIndex _result)
          (CallFunction|RandomMove))))))

(event EventBeginPlay
  ;[0.15 0.15 0.15 0.5] Comment
  (bind _returnvalue (UserInterface|CreateWidget "/Game/Blueprint/UI/WB_MainView.WB_MainView_C"))
  (Variables|Default|SetMain _returnvalue)
  (bind _asbp_patrol_point (Utilities|Casting|CastToBP_PatrolPointClass "/Game/Blueprint/PatrolPoint/BP_PatrolPoint.BP_PatrolPoint_C"))
  (bind _outactors (Actor|GetAllActorsOfClass _asbp_patrol_point))
  (bind _output_get (Variables|Default|SetPatrolPoint _outactors))
  (CallFunction|RandomMove))

(event Collision|EventActorBeginOverlap
  (params (OtherActor :type Actor%20Object%20Reference)))

(event EventTick
  (params (DeltaSeconds :type Float%20%28single-precision%29)))

(fn ConstructionScript)