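; BP_HumanCrowd moves a crowd actor along the CarSpline of a referenced track, reusing car-style naming.
; If CarOnOff is set, BeginPlay starts a timeline with its rate derived from Duration and its start time from CarStartOffset.
; The timeline's alpha maps to distance along the spline, setting the actor's world location and rotation.
; GreenLight stops the movement and RedLight resumes it, as for pedestrians opposite traffic.
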(event Custom|Move_Car
  (Components|Timeline|SetPlayRate (Variables|Default|GetCar_Mover) (/ 1.0 (Variables|Default|GetDuration)))
  (Components|Timeline|SetNewTime (Variables|Default|GetCar_Mover) (Variables|Default|GetCar_Start_Offset))
  (bind _alpha (Timeline|Car_Mover Play)
    (:Update
      (Variables|Default|SetAlpha _alpha)
      (Transformation|SetActorLocationAndRotation (Spline|GetLocationatDistanceAlongSpline (Variables|/Game/Blueprint/Station_Bravo/Blueprints/BP_Car_Track.BP_Car_Track_C|GetCar_Spline (Variables|Default|GetTrack_Reference)) (Math|Float|Lerp 0.0 (Spline|GetSplineLength (Variables|/Game/Blueprint/Station_Bravo/Blueprints/BP_Car_Track.BP_Car_Track_C|GetCar_Spline (Variables|Default|GetTrack_Reference))) (Variables|Default|GetAlpha)) "World") (Spline|GetRotationatDistanceAlongSpline (Variables|/Game/Blueprint/Station_Bravo/Blueprints/BP_Car_Track.BP_Car_Track_C|GetCar_Spline (Variables|Default|GetTrack_Reference)) (Math|Float|Lerp 0.0 (Spline|GetSplineLength (Variables|/Game/Blueprint/Station_Bravo/Blueprints/BP_Car_Track.BP_Car_Track_C|GetCar_Spline (Variables|Default|GetTrack_Reference))) (Variables|Default|GetAlpha)) "World")))))

(event Custom|RedLight
  (bind _alpha (Timeline|Car_Mover Play)
    (:Update
      (Variables|Default|SetAlpha _alpha)
      (Transformation|SetActorLocationAndRotation (Spline|GetLocationatDistanceAlongSpline (Variables|/Game/Blueprint/Station_Bravo/Blueprints/BP_Car_Track.BP_Car_Track_C|GetCar_Spline (Variables|Default|GetTrack_Reference)) (Math|Float|Lerp 0.0 (Spline|GetSplineLength (Variables|/Game/Blueprint/Station_Bravo/Blueprints/BP_Car_Track.BP_Car_Track_C|GetCar_Spline (Variables|Default|GetTrack_Reference))) (Variables|Default|GetAlpha)) "World") (Spline|GetRotationatDistanceAlongSpline (Variables|/Game/Blueprint/Station_Bravo/Blueprints/BP_Car_Track.BP_Car_Track_C|GetCar_Spline (Variables|Default|GetTrack_Reference)) (Math|Float|Lerp 0.0 (Spline|GetSplineLength (Variables|/Game/Blueprint/Station_Bravo/Blueprints/BP_Car_Track.BP_Car_Track_C|GetCar_Spline (Variables|Default|GetTrack_Reference))) (Variables|Default|GetAlpha)) "World")))))

(event Custom|GreenLight
  (bind _alpha (Timeline|Car_Mover Stop)
    (:Update
      (Variables|Default|SetAlpha _alpha)
      (Transformation|SetActorLocationAndRotation (Spline|GetLocationatDistanceAlongSpline (Variables|/Game/Blueprint/Station_Bravo/Blueprints/BP_Car_Track.BP_Car_Track_C|GetCar_Spline (Variables|Default|GetTrack_Reference)) (Math|Float|Lerp 0.0 (Spline|GetSplineLength (Variables|/Game/Blueprint/Station_Bravo/Blueprints/BP_Car_Track.BP_Car_Track_C|GetCar_Spline (Variables|Default|GetTrack_Reference))) (Variables|Default|GetAlpha)) "World") (Spline|GetRotationatDistanceAlongSpline (Variables|/Game/Blueprint/Station_Bravo/Blueprints/BP_Car_Track.BP_Car_Track_C|GetCar_Spline (Variables|Default|GetTrack_Reference)) (Math|Float|Lerp 0.0 (Spline|GetSplineLength (Variables|/Game/Blueprint/Station_Bravo/Blueprints/BP_Car_Track.BP_Car_Track_C|GetCar_Spline (Variables|Default|GetTrack_Reference))) (Variables|Default|GetAlpha)) "World")))))

(event EventBeginPlay
  (if (Variables|Default|GetCar_On/Off)
    (CallFunction|MoveCar)))

(fn ConstructionScript)